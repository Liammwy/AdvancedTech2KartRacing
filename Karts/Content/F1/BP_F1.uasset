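; BP_F1 is a drivable vehicle Blueprint, apparently an F1 car, controlled by the player.
; Enhanced Input actions for throttle, brake, handbrake and steering feed the VehicleMovementComponent, with brake and handbrake explicitly cleared on release.
; Each Tick runs a Visibility line trace with persistent debug drawing and an unused result.
; The trace end multiplies the sum of location and forward vector by 1000, so it does not point straight ahead.
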(event Input|EnhancedActionEvents|EnhancedInputActionIA_Throttle
  (params (ActionValue :type Float%20%28double-precision%29) (ElapsedSeconds :type Float%20%28double-precision%29) (TriggeredSeconds :type Float%20%28double-precision%29) (InputAction :type Input%20Action%20Object%20Reference :default "/Game/VehicleTemplate/Input/Actions/IA_Throttle.IA_Throttle"))
  (:Triggered
    (Class|ChaosVehicleMovementComponent|SetThrottleInput (Variables|Default|GetVehicleMovementComponent) ActionValue :!label _label))
  (:Completed
    (goto _label)))

(event Input|EnhancedActionEvents|EnhancedInputActionIA_Brake
  (params (ActionValue :type Float%20%28double-precision%29) (ElapsedSeconds :type Float%20%28double-precision%29) (TriggeredSeconds :type Float%20%28double-precision%29) (InputAction :type Input%20Action%20Object%20Reference :default "/Game/VehicleTemplate/Input/Actions/IA_Brake.IA_Brake"))
  (:Triggered
    (Class|ChaosVehicleMovementComponent|SetBrakeInput (Variables|Default|GetVehicleMovementComponent) ActionValue))
  (:Completed
    (Class|ChaosVehicleMovementComponent|SetBrakeInput (Variables|Default|GetVehicleMovementComponent) 0.0)))

(event Input|EnhancedActionEvents|EnhancedInputActionIA_Handbrake
  (params (ActionValue :type Boolean) (ElapsedSeconds :type Float%20%28double-precision%29) (TriggeredSeconds :type Float%20%28double-precision%29) (InputAction :type Input%20Action%20Object%20Reference :default "/Game/VehicleTemplate/Input/Actions/IA_Handbrake.IA_Handbrake"))
  (:Triggered
    (Class|ChaosVehicleMovementComponent|SetHandbrakeInput (Variables|Default|GetVehicleMovementComponent) ActionValue))
  (:Completed
    (Class|ChaosVehicleMovementComponent|SetHandbrakeInput (Variables|Default|GetVehicleMovementComponent) false)))

(event Input|EnhancedActionEvents|EnhancedInputActionIA_Steering
  (params (ActionValue :type Float%20%28double-precision%29) (ElapsedSeconds :type Float%20%28double-precision%29) (TriggeredSeconds :type Float%20%28double-precision%29) (InputAction :type Input%20Action%20Object%20Reference :default "/Game/VehicleTemplate/Input/Actions/IA_Steering.IA_Steering"))
  (:Triggered
    (Class|ChaosVehicleMovementComponent|SetSteeringInput (Variables|Default|GetVehicleMovementComponent) ActionValue :!label _label))
  (:Completed
    (goto _label)))

(event EventTick
  (params (DeltaSeconds :type Float%20%28single-precision%29))
  (bind _self self)
  (bind _returnvalue (Transformation|GetActorLocation _self))
  (Collision|LineTraceByChannel _returnvalue (* (+ _returnvalue (Transformation|GetActorForwardVector _self)) 1e+03) "TraceTypeQuery1" false 0 "Persistent"))

(fn ConstructionScript)