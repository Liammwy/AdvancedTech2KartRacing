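; Room actor with a door that swings open and shows room information when an OffroadCar_Pawn reaches it.
; DoorCollision overlap plays the DoorOpening timeline to yaw the Hinge and creates a WBP_RoomInformation widget filled with the room's number, capacity, type and image.
; End overlap reverses the timeline and removes the widget, with IsOpening guarding against repeat triggers.
; The construction script writes RoomNum onto three text renders.
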(event OnComponentBeginOverlap(doorCollision)
  (params (OverlappedComponent :type Primitive%20Component%20Object%20Reference) (OtherActor :type Actor%20Object%20Reference) (OtherComp :type Primitive%20Component%20Object%20Reference) (OtherBodyIndex :type Integer) (bFromSweep :type Boolean) (SweepResult :type Hit%20Result%20Structure%20%28by%20ref%29))
  (if (not (Variables|Default|GetisOpening))
    (Utilities|Casting|CastToOffroadCar_Pawn OtherActor)
    (CallFunction|OpenDoor)
    (Variables|Default|SetisOpening true)
    (bind _returnvalue (UserInterface|CreateWidget "/Game/UI/WBP_RoomInformation.WBP_RoomInformation_C" (Game|GetPlayerController 0)))
    (Variables|Default|SetroomInformation _returnvalue)
    (UserInterface|Viewport|AddtoViewport _returnvalue 0)
    (Default|UpdateText _returnvalue (Variables|Default|GetroomNum) (Variables|Default|GetroomCapacity) (Variables|Default|GetroomType) (Variables|Default|GetroomImage))))

(event OnComponentEndOverlap(doorCollision)
  (params (OverlappedComponent :type Primitive%20Component%20Object%20Reference) (OtherActor :type Actor%20Object%20Reference) (OtherComp :type Primitive%20Component%20Object%20Reference) (OtherBodyIndex :type Integer))
  (Utilities|Casting|CastToOffroadCar_Pawn OtherActor)
  (CallFunction|CloseDoor)
  (Widget|RemovefromParent (Variables|Default|GetroomInformation))
  (Variables|Default|SetisOpening false))

(event Custom|closeDoor
  (bind _doorrotation (Timeline|DoorOpening ReverseFromEnd)
    (:Update
      (Transformation|SetRelativeRotation (Variables|Default|Gethinge) (Math|Rotator|MakeRotator 0.0 0.0 (Math|Float|Lerp 0.0 -9e+01 _doorrotation)) false false))))

(event Custom|openDoor
  (bind _doorrotation (Timeline|DoorOpening PlayFromStart)
    (:Update
      (Transformation|SetRelativeRotation (Variables|Default|Gethinge) (Math|Rotator|MakeRotator 0.0 0.0 (Math|Float|Lerp 0.0 -9e+01 _doorrotation)) false false))))

(fn ConstructionScript
  (Rendering|Components|TextRender|SetText (Variables|Default|GetTextRender) (Variables|Default|GetroomNum))
  (Rendering|Components|TextRender|SetText (Variables|Default|GetTextRender1) (Variables|Default|GetroomNum))
  (Rendering|Components|TextRender|SetText (Variables|Default|GetTextRender2) (Variables|Default|GetroomNum)))